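; Bee enemy character that chases the player when they enter its aggro collision, stings them, then destroys itself.
; Overlap events feed a NewState state machine with Idle, Chasing, Going Back and Dying states.
; Chasing uses AI MoveTo, then lunges the capsule at the player and calls Stung on success.
; Going Back halts at the current location and idles after a delay; returning to spawn is only a debug-print placeholder.
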(event `self.CollisionAggro.OnComponentBeginOverlap`
  (params (OverlappedComponent :type "PrimitiveComponent Object Reference") (OtherActor :type "Actor Object Reference") (OtherComp :type "PrimitiveComponent Object Reference") (OtherBodyIndex :type Integer) (bFromSweep :type Boolean) (SweepResult :type "HitResult Structure (by ref)"))
  (cast `/Game/Blueprints/ThirdPersonCharacter` OtherActor)
  (`self.NewState` "NewEnumerator1"))

(event `self.CollisionAggro.OnComponentEndOverlap`
  (params (OverlappedComponent :type "PrimitiveComponent Object Reference") (OtherActor :type "Actor Object Reference") (OtherComp :type "PrimitiveComponent Object Reference") (OtherBodyIndex :type Integer))
  (cast `/Game/Blueprints/ThirdPersonCharacter` OtherActor)
  (`self.NewState` "NewEnumerator3"))

(event `NewState`
  (params (NewState :type "/Game/Blueprints/E_BeeStates Enum" :default "NewEnumerator0"))
  (switch `/Game/Blueprints/E_BeeStates` NewState ; request
    (:`NewEnumerator0`
      (switch `/Game/Blueprints/E_BeeStates` (`self.BeeState`)
        (:`NewEnumerator0`
          _)
        (:`NewEnumerator1`
          _)
        (:`NewEnumerator3`
          _))
      (set `self.BeeState` "NewEnumerator0"))
    (:`NewEnumerator1`
      (switch `/Game/Blueprints/E_BeeStates` (`self.BeeState`)
        (:`NewEnumerator0`
          _)
        (:`NewEnumerator1`
          _)
        (:`NewEnumerator3`
          _))
      (set `self.BeeState` "NewEnumerator1")
      (`|AIMoveTo` self (0.0 0.0 0.0) (`GameplayStatics.GetPlayerCharacter` 0) 1.0 true ; Follow Player
        (:`OnSuccess`
          (`KismetSystemLibrary.MoveComponentTo` (`self.CapsuleComponent`) (`self.K2_GetActorLocation` (`GameplayStatics.GetPlayerCharacter` 0)) (struct) false false 0.5) ; Attack Player
          (bind _asthird_person_character (cast `/Game/Blueprints/ThirdPersonCharacter` (`GameplayStatics.GetPlayerCharacter` 0)))
          (`/Game/Blueprints/ThirdPersonCharacter.Stung` _asthird_person_character)
          (`self.NewState` "NewEnumerator2"))))
    (:`NewEnumerator3`
      (switch `/Game/Blueprints/E_BeeStates` (`self.BeeState`)
        (:`NewEnumerator0`
          _)
        (:`NewEnumerator1`
          _)
        (:`NewEnumerator3`
          _))
      (set `self.BeeState` "NewEnumerator3")
      (`|AIMoveTo` self (`self.K2_GetActorLocation`) null 1.0 true ; Stop chasing
        (:`then`
          (`KismetSystemLibrary.Delay` 2.0)
          (`KismetSystemLibrary.PrintString` "move somewhere") ; Return to spawn location
          (`self.NewState` "NewEnumerator0"))))
    (:`NewEnumerator2`
      (set `self.BeeState` "NewEnumerator2")
      (`self.K2_DestroyActor`))))

(fn `UserConstructionScript`)