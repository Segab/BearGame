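; Bee enemy character that chases the player's bear and sacrifices itself when it attacks.
; Aggro and attack collision overlaps with the bear request changes in an enum state machine (Idle, Chasing, Attack, Going Back, Dying).
; Chasing scales walk speed from the bear's BeeAggression.
; Attacking puts the bear in a new state and destroys the bee, while Going Back drops straight to Idle.
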(event `self.ReceiveBeginPlay`
  ;[1 1 1] Store Max Walk Speed
  (set `self.BaseWalkSpeed` (`CharacterMovementComponent.MaxWalkSpeed` (`self.CharacterMovement`))))

(event `self.CollisionAggro.OnComponentBeginOverlap`
  (params (OverlappedComponent :type "PrimitiveComponent Object Reference") (OtherActor :type "Actor Object Reference") (OtherComp :type "PrimitiveComponent Object Reference") (OtherBodyIndex :type Integer) (bFromSweep :type Boolean) (SweepResult :type "HitResult Structure (by ref)"))
  ;[1 1 1] Bee Aggro Range Triggers
  (cast `/Game/Blueprints/Bear/BearCharacterBP` OtherActor)
  (`self.NewState` "NewEnumerator1"))

(event `self.CollisionAggro.OnComponentEndOverlap`
  (params (OverlappedComponent :type "PrimitiveComponent Object Reference") (OtherActor :type "Actor Object Reference") (OtherComp :type "PrimitiveComponent Object Reference") (OtherBodyIndex :type Integer))
  ;[1 1 1] Bee Aggro Range Triggers
  (cast `/Game/Blueprints/Bear/BearCharacterBP` OtherActor)
  (`self.NewState` "NewEnumerator3"))

(event `self.CollisionAttack.OnComponentBeginOverlap`
  (params (OverlappedComponent :type "PrimitiveComponent Object Reference") (OtherActor :type "Actor Object Reference") (OtherComp :type "PrimitiveComponent Object Reference") (OtherBodyIndex :type Integer) (bFromSweep :type Boolean) (SweepResult :type "HitResult Structure (by ref)"))
  ;[1 1 1] Bee Aggro Range Triggers
  (cast `/Game/Blueprints/Bear/BearCharacterBP` OtherActor)
  (`self.NewState` "NewEnumerator4"))

(event `NewState`
  (params (NewState :type "/Game/Blueprints/Bees/E_BeeStates Enum" :default "NewEnumerator0"))
  (switch `/Game/Blueprints/Bees/E_BeeStates` NewState ; request
    (:`NewEnumerator0`
      (switch `/Game/Blueprints/Bees/E_BeeStates` (`self.BeeState`)
        (:`NewEnumerator0`
          _)
        (:`NewEnumerator1`
          _)
        (:`NewEnumerator3`
          _))
      (set `self.BeeState` "NewEnumerator0"))
    (:`NewEnumerator1`
      (switch `/Game/Blueprints/Bees/E_BeeStates` (`self.BeeState`)
        (:`NewEnumerator0`
          _)
        (:`NewEnumerator1`
          _)
        (:`NewEnumerator3`
          _))
      (set `self.BeeState` "NewEnumerator1")
      (`self.CalcBeeSpeed`))
    (:`NewEnumerator4`
      (switch `/Game/Blueprints/Bees/E_BeeStates` (`self.BeeState`)
        (:`NewEnumerator1`
          _)
        (:`NewEnumerator4`
          _))
      (set `self.BeeState` "NewEnumerator4")
      (bind _asbear_character_bp (cast `/Game/Blueprints/Bear/BearCharacterBP` (`GameplayStatics.GetPlayerCharacter` 0)))
      (`/Game/Blueprints/Bear/BearCharacterBP.NewState` _asbear_character_bp "NewEnumerator4") ; Bear enters hit state
      (`self.NewState` "NewEnumerator2") ; Bee enters dying state
    )
    (:`NewEnumerator3`
      (switch `/Game/Blueprints/Bees/E_BeeStates` (`self.BeeState`)
        (:`NewEnumerator0`
          _)
        (:`NewEnumerator1`
          _)
        (:`NewEnumerator3`
          _))
      (set `self.BeeState` "NewEnumerator3")
      (`self.NewState` "NewEnumerator0"))
    (:`NewEnumerator2`
      (set `self.BeeState` "NewEnumerator2")
      (`self.K2_DestroyActor`))))

(fn `CalcBeeSpeed`
  (bind _asbear_character_bp (cast `/Game/Blueprints/Bear/BearCharacterBP` (`GameplayStatics.GetPlayerCharacter` 0)))
  (set `CharacterMovementComponent.MaxWalkSpeed` (* (+ (* (`/Game/Blueprints/Bear/BearCharacterBP.BeeAggression` _asbear_character_bp) 0.0075) 0.25) (`self.BaseWalkSpeed`)) (`self.CharacterMovement`)))

(fn `UserConstructionScript`)