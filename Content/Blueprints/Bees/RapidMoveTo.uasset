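; Behavior Tree task that moves a bee AI's controlled pawn to a target actor.
; On execute, it casts the owner to BeesAIController, reads the TargetToFollow blackboard actor and runs an async AI MoveTo with a tight acceptance radius.
; The move result finishes the task as success or failure, with debug prints on start and outcome.
; A failed controller cast leaves the task without a finish call.
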(event `self.ReceiveExecute`
  (params (OwnerActor :type "Actor Object Reference"))
  (bind _asbees_aicontroller (cast `/Game/Blueprints/Bees/BeesAIController` OwnerActor))
  (set `self.BeeConRef` _asbees_aicontroller)
  (`|AIMoveTo` (`Controller.K2_GetPawn` (`self.BeeConRef`)) (0.0 0.0 0.0) (`BTFunctionLibrary.GetBlackboardValueAsActor` (`self.Target to Follow`)) 50.0
    (:`then`
      (`KismetSystemLibrary.PrintString` "start task" true true (struct :`R` 1.0 :`G` 0.034921 :`A` 1.0) 5.0))
    (:`OnSuccess`
      (`self.FinishExecute` true)
      (`KismetSystemLibrary.PrintString` "Success" true true (struct :`R` 1.0 :`G` 0.025803 :`A` 1.0)))
    (:`OnFail`
      (`self.FinishExecute` false)
      (`KismetSystemLibrary.PrintString` "Fiail" true true (struct :`R` 1.0 :`G` 0.149544 :`A` 1.0)))))