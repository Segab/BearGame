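; FarEnough is a behavior tree decorator for the bee AI that checks whether a bee is far enough from the target it follows, noted as the player.
; Its condition check casts the owner to BeesAIController and reads the TargetToFollow actor from the Blackboard.
; It passes when the distance between that actor and the controlled pawn is at least AcceptableDistance.
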(fn `PerformConditionCheck`
  (params (OwnerActor :type "Actor Object Reference"))
  (returns (ReturnValue :type Boolean))
  (bind _asbees_aicontroller (cast `/Game/Blueprints/Bees/BeesAIController` OwnerActor))
  (set `self.BeesConRef` _asbees_aicontroller)
  (return (>= (`KismetMathLibrary.VSize` (- (`Actor.K2_GetActorLocation` (`BTFunctionLibrary.GetBlackboardValueAsActor` (`self.TargetToFollow`))) (`Actor.K2_GetActorLocation` (`Controller.K2_GetPawn` (`self.BeesConRef`))))) (`self.AcceptableDistance`))))