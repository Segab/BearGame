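; AI controller for bee characters that runs the BeesBT behavior tree and makes the bee jump at obstacles.
; On begin play it sets up the BeesBB blackboard with the player character as a key, then starts the tree.
; It stores the possessed Character and, each tick while that moves fast enough, sphere-traces ahead on Visibility, jumping on a hit.
; The trace leaves persistent debug drawing enabled.
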(event `self.ReceiveBeginPlay`
  (bind _blackboardcomponent (`self.UseBlackboard` "/Game/Blueprints/BeesBB.BeesBB"))
  (`BlackboardComponent.SetValueAsObject` _blackboardcomponent (`self.PlayerCharKey`) (`GameplayStatics.GetPlayerCharacter` 0))
  (`self.RunBehaviorTree` "/Game/Blueprints/BeesBT.BeesBT"))

(event `self.OnPossess`
  (params (PossessedPawn :type "Pawn Object Reference"))
  (bind _ascharacter (cast `Character` PossessedPawn))
  (set `self.StoredPawn` _ascharacter))

(event `self.ReceiveTick`
  (params (DeltaSeconds :type "Float (single-precision)"))
  (bind _storedpawn (`self.StoredPawn`))
  (bind _returnvalue (`self.K2_GetActorLocation` _storedpawn))
  (if (>= (`KismetMathLibrary.VSize` (`self.GetVelocity` (`self.StoredPawn`))) 100.0)
    (bind (_outhits _returnvalue_2) (`KismetSystemLibrary.SphereTraceMulti` _returnvalue (+ _returnvalue (* (`self.GetActorForwardVector` _storedpawn) 250.0)) 0.0 "TraceTypeQuery1" true (`|MakeArray` (`self.StoredPawn`) :!type "Actor Object Reference") "Persistent"))
    (if _returnvalue_2
      (`Character.Jump` (`self.StoredPawn`)))))

(fn `UserConstructionScript`)